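; BP_EnemySpawner is an actor that repeatedly spawns BP_EnemyCharger enemies at its own root location.
; Tick feeds a five-second Delay, so a new AI pawn appears roughly every five seconds.
; Each spawned charger receives the spawner's Id, which also indexes the Materials array to set the material on its three cube meshes.
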(event EventTick
  (params (DeltaSeconds :type Float%20%28single-precision%29))
  ;[1 1 1] Spawn Enemy
  (Utilities|FlowControl|Delay 5.0)
  (bind _returnvalue (AI|SpawnAIFromClass "/Game/J-M/BluePrintJ-M/BP_EnemyCharger.BP_EnemyCharger_C" 0 (Transformation|GetWorldLocation (Variables|Default|GetDefaultSceneRoot)) "0, 0, 0" false 0))
  (bind _asbp_enemy_charger (Utilities|Casting|CastToBP_EnemyCharger _returnvalue))
  (Variables|/Game/J-M/BluePrintJ-M/BP_EnemyCharger.BP_EnemyCharger_C|Setid _asbp_enemy_charger (Variables|Default|Getid))
  (Rendering|Material|SetMaterial (Variables|/Game/J-M/BluePrintJ-M/BP_EnemyCharger.BP_EnemyCharger_C|GetCube _asbp_enemy_charger) 0 (Utilities|Array|Get(acopy) (Variables|Default|Getmaterials) (Variables|Default|Getid))))

(fn ConstructionScript)